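; BP_PortalPassword is a password puzzle that reveals a hidden sphere when a set of count boxes matches a code.
; On BeginPlay it hides the Sphere and binds to the FClick dispatcher of each box in Counts.
; FuncPressFClick sets Sphere visibility from IsAllBox9, which, despite its name, compares each box's Count to the Password entry at the same index.
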(event `self.ReceiveBeginPlay`
  (`SceneComponent.SetVisibility` (`self.Sphere`) false false)
  ; Count박스 이벤트 바인딩
  (for _array_element (`self.Counts`)
    (add `/Game/BlueprintEX/BP_Counting.EventDispatcher_FClick` _array_element (`|CreateDelegate` :!event `FuncPressFClick`))))

(fn `FuncPressFClick`
  (`KismetSystemLibrary.PrintString` "FuncPressFClick")
  (`SceneComponent.SetVisibility` (`self.Sphere`) (`self.IsAllBox9`) false))

(fn `IsAllBox9`
  (returns (AllBox9 :type Boolean))
  (for (_array_element _array_index) (`self.Counts`)
    (if (not (== (`/Game/BlueprintEX/BP_Counting.Count` _array_element) (`|GetArrayItem` (`self.Password`) _array_index)))
      (return false)))
  (return true))

(fn `UserConstructionScript`)