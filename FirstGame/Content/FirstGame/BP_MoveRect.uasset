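; BP_MoveRect is an Actor Blueprint that moves its Cube component around a square path in the local XZ plane.
; Tick switches on the MoveType state, cycling Right, Up, Left and Down as each position limit is reached.
; Each state steps the stored X or Z value by a fixed amount and applies it as the Cube's relative location.
; The step ignores delta time, so speed depends on frame rate.
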(event `self.ReceiveTick`
  (params (DeltaSeconds :type "Float (single-precision)"))
  (switch `/Game/FirstGame/ENUM_MoveType` (`self.MoveType`)
    (:`NewEnumerator0`
      ; 오른쪽으로 이동한다.
      ;; X의 위치에 2을 더한다
      (set `self.X의 위치` (+ (`self.X의 위치`) 2.0))
      ;; Box에 상대좌표 X를 "X의 위치"값으로 변경한다.
      (`SceneComponent.K2_SetRelativeLocation` (`self.Cube`) (`KismetMathLibrary.MakeVector` (`self.X의 위치`) 0.0 (`self.Z의 위치`)) false false)
      (if (>= (`self.X의 위치`) 500.0)
        (set `self.MoveType` "NewEnumerator1")))
    (:`NewEnumerator1`
      ; 위쪽으로 이동
      ;; Z의 위치에 2을 더한다
      (set `self.Z의 위치` (+ (`self.Z의 위치`) 2.0))
      ;; Box에 상대좌표 Z를 "Z의 위치"값으로 변경한다.
      (`SceneComponent.K2_SetRelativeLocation` (`self.Cube`) (`KismetMathLibrary.MakeVector` (`self.X의 위치`) 0.0 (`self.Z의 위치`)) false false)
      (if (>= (`self.Z의 위치`) 500.0)
        (set `self.MoveType` "NewEnumerator2")))
    (:`NewEnumerator2`
      ; 왼쪽으로 이동한다.
      ;; X의 위치에 2을 뺀다
      (set `self.X의 위치` (- (`self.X의 위치`) 2.0))
      ;; Box에 상대좌표 X를 "X의 위치"값으로 변경한다.
      (`SceneComponent.K2_SetRelativeLocation` (`self.Cube`) (`KismetMathLibrary.MakeVector` (`self.X의 위치`) 0.0 (`self.Z의 위치`)) false false)
      (if (<= (`self.X의 위치`) 0.0)
        (set `self.MoveType` "NewEnumerator3")))
    (:`NewEnumerator3`
      ; 위쪽으로 이동
      ;; Z의 위치에 2을 뺀다
      (set `self.Z의 위치` (- (`self.Z의 위치`) 2.0))
      ;; Box에 상대좌표 Z를 "Z의 위치"값으로 변경한다.
      (`SceneComponent.K2_SetRelativeLocation` (`self.Cube`) (`KismetMathLibrary.MakeVector` (`self.X의 위치`) 0.0 (`self.Z의 위치`)) false false)
      (if (<= (`self.Z의 위치`) 0.0)
        (set `self.MoveType` "NewEnumerator0")))))

(fn `UserConstructionScript`)