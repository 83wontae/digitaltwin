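; BP_SwitchArea is a trigger area that fires two spawners when something begins overlapping its Cube.
; The overlap runs a Sequence of two loops that call DoSpawn repeatedly on Spawner1, then on Spawner2, with no filter or one-shot guard.
; The construction script labels the TextRender with the actor's display name.
; Unconnected loop nodes remain, one with a Korean note explaining ForLoop behavior.
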(event `self.Cube.OnComponentBeginOverlap`
  (params (OverlappedComponent :type "PrimitiveComponent Object Reference") (OtherActor :type "Actor Object Reference") (OtherComp :type "PrimitiveComponent Object Reference") (OtherBodyIndex :type Integer) (bFromSweep :type Boolean) (SweepResult :type "HitResult Structure (by ref)"))
  (`|ExecutionSequence`
    (:`then_0`
      (for _ (range 11)
        (`/Game/FirstGame/BP_SpawnArea.DoSpawn` (`self.Spawner1`))))
    (:`then_1`
      (for _ (range 6)
        (`/Game/FirstGame/BP_SpawnArea.DoSpawn` (`self.Spawner2`))))))

(fn `UserConstructionScript`
  (`TextRenderComponent.K2_SetText` (`self.TextRender`) (`KismetTextLibrary.Conv_StringToText` (`KismetSystemLibrary.GetDisplayName` self))))