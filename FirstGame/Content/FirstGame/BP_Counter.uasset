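; BP_Counter is a counter actor that counts down on a text display each time something begins overlapping its Cube.
; BeginPlay writes the initial value to the TextRender component.
; Each overlap increments Count, wraps it to zero once it passes nine, and refreshes the text.
; The display shows nine minus Count, so the visible number falls to zero and then restarts at nine.
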(event `self.ReceiveBeginPlay`
  (`TextRenderComponent.K2_SetText` (`self.TextRender`) (`KismetTextLibrary.Conv_IntToText` (- 9 (`self.Count`)))))

(event `self.Cube.OnComponentBeginOverlap`
  (params (OverlappedComponent :type "PrimitiveComponent Object Reference") (OtherActor :type "Actor Object Reference") (OtherComp :type "PrimitiveComponent Object Reference") (OtherBodyIndex :type Integer) (bFromSweep :type Boolean) (SweepResult :type "HitResult Structure (by ref)"))
  ; Count 를 1증가
  (set `self.Count` (+ (`self.Count`) 1))
  ; count가 9보다 크면
  (if (> (`self.Count`) 9)
    ; Count 0으로 변경
    (set `self.Count` 0))
  ; Count 를 Text Render에 표시
  (`TextRenderComponent.K2_SetText` (`self.TextRender`) (`KismetTextLibrary.Conv_IntToText` (- 9 (`self.Count`)))))

(fn `UserConstructionScript`)