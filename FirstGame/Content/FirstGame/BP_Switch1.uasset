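; BP_Switch1 is an overlap-triggered switch actor that tells a referenced Abc object to spawn when something enters its Cube component.
; Begin overlap prints the overlapped component, other actor and other component names for debugging, then calls DoSpawn on Abc; end overlap only prints a message.
; The construction script labels the switch by setting its TextRender to the actor's own display name.
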(event `self.Cube.OnComponentBeginOverlap`
  (params (OverlappedComponent :type "PrimitiveComponent Object Reference") (OtherActor :type "Actor Object Reference") (OtherComp :type "PrimitiveComponent Object Reference") (OtherBodyIndex :type Integer) (bFromSweep :type Boolean) (SweepResult :type "HitResult Structure (by ref)"))
  (`KismetSystemLibrary.PrintString` (`KismetStringLibrary.Concat_StrStr` "Begin Overlap " "Overlapped Component : " (`KismetSystemLibrary.GetDisplayName` OverlappedComponent) ", Other Actor : " (`KismetSystemLibrary.GetDisplayName` OtherActor) ", Other Comp : " (`KismetSystemLibrary.GetDisplayName` OtherComp)) true true (struct :`G` 0.66 :`B` 1.0 :`A` 1.0) 60.0)
  (`/Game/FirstGame/BP_SpawnArea.DoSpawn` (`self.abc`)))

(event `self.Cube.OnComponentEndOverlap`
  (params (OverlappedComponent :type "PrimitiveComponent Object Reference") (OtherActor :type "Actor Object Reference") (OtherComp :type "PrimitiveComponent Object Reference") (OtherBodyIndex :type Integer))
  (`KismetSystemLibrary.PrintString` "End Overlap"))

(fn `UserConstructionScript`
  (`TextRenderComponent.K2_SetText` (`self.TextRender`) (`KismetTextLibrary.Conv_StringToText` (`KismetSystemLibrary.GetDisplayName` self))))