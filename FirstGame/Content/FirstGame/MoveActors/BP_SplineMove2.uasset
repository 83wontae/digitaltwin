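; BP_SplineMove2 is an actor that moves a Cube back and forth along its Spline.
; A timeline scales its value by the spline length and sets the cube's world location to that distance along the path, without changing rotation or sweeping.
; BeginPlay plays or reverses the timeline based on IsRight, and each finish flips that flag and re-runs the check to keep the ping-pong going.
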(event `self.ReceiveBeginPlay`
  (bind _spline (`self.Spline`))
  (if (`self.IsRight`) :!label _label
    (bind (_direction _value) (`Timeline|타임라인` :!label _label_2)
      (:`Update`
        (bind _returnvalue_location (`KismetMathLibrary.BreakTransform` (`SplineComponent.GetTransformAtDistanceAlongSpline` _spline (* _value (`SplineComponent.GetSplineLength` _spline)) "World" false)))
        (`SceneComponent.K2_SetWorldLocation` (`self.Cube`) _returnvalue_location false false))
      (:`Finished`
        (set `self.IsRight` (not (`self.IsRight`)))
        (goto _label)))
    (else
      (goto _label_2 :!via `Reverse`))))

(fn `UserConstructionScript`)