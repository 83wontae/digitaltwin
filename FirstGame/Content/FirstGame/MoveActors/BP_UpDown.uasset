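; BP_UpDown is an actor whose static mesh bobs up and down while it is switched on.
; Each Tick nudges the mesh's relative Z by a fixed step, flipping IsMoveUp when it passes the upper or lower limit.
; The step is per frame rather than scaled by delta time, so speed depends on frame rate.
; DoPlayAndStop sets the IsPlay flag that starts or pauses the motion.
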(event `self.ReceiveTick`
  (params (DeltaSeconds :type "Float (single-precision)"))
  (bind (_relativelocation_x _relativelocation_y _relativelocation_z) (`KismetMathLibrary.BreakVector` (`SceneComponent.RelativeLocation` (`self.StaticMesh`))))
  (bind (_relativelocation_x_2 _relativelocation_y_2 _relativelocation_z_2) (`KismetMathLibrary.BreakVector` (`SceneComponent.RelativeLocation` (`self.StaticMesh`))))
  (if (`self.IsPlay`)
    (if (`self.IsMoveUp`)
      (`SceneComponent.K2_AddRelativeLocation` (`self.StaticMesh`) (0.0 0.0 10.0) false false)
      (if (> _relativelocation_z_2 500.0)
        (set `self.IsMoveUp` false))
      (else
        (`SceneComponent.K2_AddRelativeLocation` (`self.StaticMesh`) (0.0 0.0 -10.0) false false)
        (if (< _relativelocation_z 0.0)
          (set `self.IsMoveUp` true))))))

(fn `DoPlayAndStop`
  (params (IsPlay :type Boolean))
  (returns (bResult :type Boolean))
  (set `self.IsPlay` IsPlay)
  (return false))

(fn `UserConstructionScript`)