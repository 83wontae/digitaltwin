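; BP_LeftRight is a moving actor whose Box component shuttles back and forth along its relative X axis while IsPlay is true.
; Each Tick steps X의위치 (X position) by a fixed amount, without delta-time scaling, so speed depends on frame rate.
; The 오른쪽이동인가 (moving right) flag selects the direction and flips at the 0 and 500 limits.
; Inline comments claim a step of 100, but the code uses 10.
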(event `self.ReceiveTick`
  (params (DeltaSeconds :type "Float (single-precision)"))
  (if (`self.IsPlay`)
    (if (`self.오른쪽 이동인가?`)
      ; 오른쪽으로 이동한다.
      ;; X의 위치에 100을 더한다
      (set `self.X의 위치` (+ (`self.X의 위치`) 10.0))
      ;; Box에 상대좌표 X를 "X의 위치"값으로 변경한다.
      (`SceneComponent.K2_SetRelativeLocation` (`self.Box`) (`KismetMathLibrary.MakeVector` (`self.X의 위치`)) false false)
      (if (>= (`self.X의 위치`) 500.0)
        (set `self.오른쪽 이동인가?` false))
      (else
        ; 왼쪽으로 이동한다.
        ;; X의 위치에 100을 더한다
        (set `self.X의 위치` (- (`self.X의 위치`) 10.0))
        ;; Box에 상대좌표 X를 "X의 위치"값으로 변경한다.
        (`SceneComponent.K2_SetRelativeLocation` (`self.Box`) (`KismetMathLibrary.MakeVector` (`self.X의 위치`)) false false)
        (if (<= (`self.X의 위치`) 0.0)
          (set `self.오른쪽 이동인가?` true))))))

(fn `UserConstructionScript`)